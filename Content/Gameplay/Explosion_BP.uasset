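; Short-lived explosion actor that applies a physics blast and damages a bot.
; On BeginPlay it fires its RadialForce impulse, sets a brief lifespan and caches the first Bot2 found in the level.
; Sphere begin-overlap calls RocketDamage only when the overlapping actor is that cached Bot2, so other Bot2 instances take no damage from it.
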(event OnComponentBeginOverlap(Sphere)
  (params (OverlappedComponent :type Primitive%20Component%20Object%20Reference) (OtherActor :type Actor%20Object%20Reference) (OtherComp :type Primitive%20Component%20Object%20Reference) (OtherBodyIndex :type Integer) (bFromSweep :type Boolean) (SweepResult :type Hit%20Result%20Structure%20%28by%20ref%29))
  (bind _as_bot_2 (Variables|Default|GetAs%20Bot%202))
  (if (== OtherActor _as_bot_2)
    (Default|RocketDamage _as_bot_2)))

(event EventBeginPlay
  (Class|RadialForceComponent|FireImpulse (Variables|Default|GetRadialForce))
  (Actor|SetLifeSpan 3.0)
  (bind _outactors (Actor|GetAllActorsOfClass "/Game/NPC4/Bot2.Bot2_C"))
  (bind _asbot_2 (Utilities|Casting|CastToBot2 (Utilities|Array|Get(acopy) _outactors)))
  (Variables|Default|SetAs%20Bot%202 _asbot_2))

(fn ConstructionScript)